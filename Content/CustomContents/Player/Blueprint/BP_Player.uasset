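; BP_Player is the player character, handling Enhanced Input movement, pickups, an AK47 equip toggle, damage montages and timeline-driven aim zoom.
; Stat, inventory and quick-slot components hold state, which is pushed to the controller's HUD.
; Quick-slot use reads item DataTables, heals, draws from the smallest inventory stack, and clears all quick slots when that item runs out.
; A helper converts the weapon's LeftHandIK socket into right-hand bone space.
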(event `self.ReceiveBeginPlay`
  (bind _asbp_player_controller (cast `/Game/CustomContents/Player/Blueprint/BP_PlayerController` (`self.GetController`)))
  (bind _output_get (set `self.PlayerController` _asbp_player_controller))
  (`EnhancedInputSubsystemInterface.AddMappingContext` (pcsubsystem `EnhancedInputLocalPlayerSubsystem` _output_get) "/Game/CustomContents/Player/Inputs/IMC_Player.IMC_Player" 0 (struct))
  (`self.InitializeQuickSlot`))

(event `EnhancedInput|/Game/CustomContents/Player/Inputs/IA/IA_PutOnWeapon`
  (params (ActionValue :type Boolean) (ElapsedSeconds :type "Float (double-precision)") (TriggeredSeconds :type "Float (double-precision)") (InputAction :type "InputAction Object Reference" :default "/Game/CustomContents/Player/Inputs/IA/IA_PutOnWeapon.IA_PutOnWeapon"))
  ;[1 1 1] PutOnWeponInput
  (:`Started`
    (`/Engine/EditorBlueprintResources/StandardMacros.FlipFlop`
      (:`A`
        (`/Engine/EditorBlueprintResources/StandardMacros.IsValid` (`self.AK47`)
          (:`Is Valid`
            (if (not (`self.IsArmedRifle`))
              (bind _returnvalue (`|GetDataTableRow` "/Game/CustomContents/Items/Weapons/DT_Weapon.DT_Weapon" "AK47")
                (:`then`
                  (bind _returnvalue_2 (`|SpawnActorFromClass` (`.WeaponClass_11_041DB66D4B8BB26AA0FEE8B97D280C16` (break `/Game/CustomContents/Items/Weapons/S_Weapon` _returnvalue)) (`KismetMathLibrary.MakeTransform` (0.0 0.0 0.0)) "Undefined" "MultiplyWithRoot" null null))
                  (bind _output_get (set `self.Weapon` _returnvalue_2))
                  (bind _returnvalue_3 (`self.K2_AttachToComponent` _output_get (`self.Mesh`) "AK47" "KeepRelative" "KeepRelative" "KeepRelative" true))
                  (set `self.IsArmedRifle` _returnvalue_3)
                  (`TextBlock.SetText` (`/Game/CustomContents/UI/WB_HUD.ItemName` (`/Game/CustomContents/Player/Blueprint/BP_PlayerController.PlayerHUD` (`self.PlayerController`))) "")))))))
      (:`B`
        (`StaticMeshComponent.SetStaticMesh` (`self.AK47`) (`self.New Mesh`))
        (set `self.IsArmedRifle` false)
        (`self.K2_DestroyActor` (`self.Weapon`))))))

(event `EnhancedInput|/Game/CustomContents/Player/Inputs/IA/IA_LookAround`
  (params (ActionValue :type "Vector2D Structure") (ElapsedSeconds :type "Float (double-precision)") (TriggeredSeconds :type "Float (double-precision)") (InputAction :type "InputAction Object Reference" :default "/Game/CustomContents/Player/Inputs/IA/IA_LookAround.IA_LookAround"))
  ;[1 1 1] LookAroundInput
  (:`Triggered`
    (`self.AddControllerYawInput` (`KismetMathLibrary.FClamp` ActionValue_X -3.0 3.0))
    (`self.AddControllerPitchInput` (`KismetMathLibrary.FClamp` (* ActionValue_Y -1.0) -0.3 0.3))))

(event `EnhancedInput|/Game/CustomContents/Player/Inputs/IA/IA_Movement`
  (params (ActionValue :type "Vector2D Structure") (ElapsedSeconds :type "Float (double-precision)") (TriggeredSeconds :type "Float (double-precision)") (InputAction :type "InputAction Object Reference" :default "/Game/CustomContents/Player/Inputs/IA/IA_Movement.IA_Movement"))
  (bind (_returnvalue_roll _returnvalue_pitch _returnvalue_yaw) (`KismetMathLibrary.BreakRotator` (`self.GetControlRotation`)))
  (bind (_returnvalue_roll_2 _returnvalue_pitch_2 _returnvalue_yaw_2) (`KismetMathLibrary.BreakRotator` (`self.GetControlRotation`)))
  ;[1 1 1] MovementInput
  (:`Triggered`
    (if (not (`self.IsHitting`))
      (`self.AddMovementInput` (`KismetMathLibrary.GetRightVector` (`KismetMathLibrary.MakeRotator` _returnvalue_roll_2 0.0 _returnvalue_yaw_2)) ActionValue_X)
      (`self.AddMovementInput` (`KismetMathLibrary.GetForwardVector` (`KismetMathLibrary.MakeRotator` 0.0 0.0 _returnvalue_yaw)) ActionValue_Y))))

(event `EnhancedInput|/Game/CustomContents/Player/Inputs/IA/IA_Sprint`
  (params (ActionValue :type Boolean) (ElapsedSeconds :type "Float (double-precision)") (TriggeredSeconds :type "Float (double-precision)") (InputAction :type "InputAction Object Reference" :default "/Game/CustomContents/Player/Inputs/IA/IA_Sprint.IA_Sprint"))
  (bind _charactermovement (`self.CharacterMovement`))
  ;[1 1 1] SprintInput (달리기)
  (:`Triggered`
    (set `CharacterMovementComponent.MaxWalkSpeed` 600.0 _charactermovement) ; 달리는 속력
    (set `self.isSpring` true))
  (:`Completed`
    (set `CharacterMovementComponent.MaxWalkSpeed` 450.0 _charactermovement) ; 걷는 속력
    (set `self.isSpring` false)))

(event `EnhancedInput|/Game/CustomContents/Player/Inputs/IA/IA_Jump`
  (params (ActionValue :type Boolean) (ElapsedSeconds :type "Float (double-precision)") (TriggeredSeconds :type "Float (double-precision)") (InputAction :type "InputAction Object Reference" :default "/Game/CustomContents/Player/Inputs/IA/IA_Jump.IA_Jump"))
  ;[1 1 1] JumpInput
  (:`Started`
    (`self.Jump`))
  (:`Completed`
    (`self.StopJumping`)))

(event `EnhancedInput|/Game/CustomContents/Player/Inputs/IA/IA_Crouch`
  (params (ActionValue :type Boolean) (ElapsedSeconds :type "Float (double-precision)") (TriggeredSeconds :type "Float (double-precision)") (InputAction :type "InputAction Object Reference" :default "/Game/CustomContents/Player/Inputs/IA/IA_Crouch.IA_Crouch"))
  ;[1 1 1] Crouch
  (:`Started`
    (`/Engine/EditorBlueprintResources/StandardMacros.FlipFlop`
      (:`A`
        (`self.Crouch`))
      (:`B`
        (`self.UnCrouch`)))))

(event `EnhancedInput|/Game/CustomContents/Player/Inputs/IA/IA_PickUpOrange`
  (params (ActionValue :type Boolean) (ElapsedSeconds :type "Float (double-precision)") (TriggeredSeconds :type "Float (double-precision)") (InputAction :type "InputAction Object Reference" :default "/Game/CustomContents/Player/Inputs/IA/IA_PickUpOrange.IA_PickUpOrange"))
  (bind _icon (`self.Icon`))
  (bind _returnvalue (`self.GetComponentByClass` _icon "/Game/CustomContents/Components/BPC_Item.BPC_Item_C"))
  (bind (_datatable _rowname) (break `DataTableRowHandle` (`/Game/CustomContents/Components/BPC_Item.ItemData` _returnvalue)))
  ;[1 1 1] PickUpInput
  (:`Started`
    (`/Engine/EditorBlueprintResources/StandardMacros.IsValid` _icon
      (:`Is Valid`
        (bind _returnvalue_2 (`|GetDataTableRow` _datatable _rowname)
          (:`then`
            (switch `/Game/CustomContents/Items/E_ItemType` (`.ItemType_14_F5EEFD9146030F0D2F3A7A8BDA3BBCE4` (break `/Game/CustomContents/Items/ItemBlueprints/S_Item` _returnvalue_2))
              (:`NewEnumerator4`
                (message `/Game/CustomContents/Inventory/Blueprint/BPI_Interact.Interact` _returnvalue self)
                (`self.UpdateInventory`)))))))))

(event `EnhancedInput|/Game/CustomContents/Player/Inputs/IA/IA_PickUpSkill`
  (params (ActionValue :type Boolean) (ElapsedSeconds :type "Float (double-precision)") (TriggeredSeconds :type "Float (double-precision)") (InputAction :type "InputAction Object Reference" :default "/Game/CustomContents/Player/Inputs/IA/IA_PickUpSkill.IA_PickUpSkill"))
  ;[1 1 1] PickUpInput
  (:`Started`
    (`self.DepreciatedAddItem`)))

(event `EnhancedInput|/Game/CustomContents/Player/Inputs/IA/IA_QuickSlot1`
  (params (ActionValue :type Boolean) (ElapsedSeconds :type "Float (double-precision)") (TriggeredSeconds :type "Float (double-precision)") (InputAction :type "InputAction Object Reference" :default "/Game/CustomContents/Player/Inputs/IA/IA_QuickSlot1.IA_QuickSlot1"))
  ;[1 1 1] QuickSlotInput
  (:`Started`
    (bind _output_get (set `self.PressedQuickSlotIndex` 0))
    (`self.UseItem` _output_get)))

(event `UpdateInventory`
  (bind _wb_menu (`/Game/CustomContents/UI/WB_HUD.WB_Menu` (`/Game/CustomContents/Player/Blueprint/BP_PlayerController.PlayerHUD` (`self.PlayerController`))))
  (`/Engine/EditorBlueprintResources/StandardMacros.IsValid` _wb_menu
    (:`Is Valid`
      (`/Game/CustomContents/UI/Inventory/WB_Inventory.UpdateInventory` (`/Game/CustomContents/UI/Inventory/WB_InventoryMenu.WB_Inventory` _wb_menu) (`self.BPC_InventorySystem`)))))

(event `self.ReceiveAnyDamage`
  (params (Damage :type "Float (single-precision)") (DamageType :type "DamageType Object Reference") (InstigatedBy :type "Controller Object Reference") (DamageCauser :type "Actor Object Reference"))
  ;[1 1 1] HitDamage
  (set `self.IsHitting` true)
  (bind _isdead (`/Game/CustomContents/Components/BPC_StatSystem.DecreaseHealth` (`self.BPC_StatSystem`) Damage (`/Game/CustomContents/Player/Blueprint/BP_PlayerController.PlayerHUD` (`self.PlayerController`))))
  (if _isdead
    (`|PlayMontage` (`self.Mesh`) "/Game/CustomContents/Animations/Montage/Death_Montage.Death_Montage"
      (:`then`
        (`PrimitiveComponent.SetCollisionEnabled` (`self.CapsuleComponent`) "NoCollision"))
      (:`OnCompleted`
        (set `self.IsHitting` false)))
    (else
      (`|PlayMontage` (`self.Mesh`) "/Game/CustomContents/Animations/Montage/Hit_1_Montage.Hit_1_Montage"
        (:`OnCompleted`
          (set `self.IsHitting` false))))))

(event `EnhancedInput|/Game/CustomContents/Player/Inputs/IA/IA_QuickSlot2`
  (params (ActionValue :type Boolean) (ElapsedSeconds :type "Float (double-precision)") (TriggeredSeconds :type "Float (double-precision)") (InputAction :type "InputAction Object Reference" :default "/Game/CustomContents/Player/Inputs/IA/IA_QuickSlot2.IA_QuickSlot2"))
  ;[1 1 1] QuickSlotInput
  (:`Started`
    (bind _output_get (set `self.PressedQuickSlotIndex` 1))
    (`self.UseItem` _output_get)))

(event `InitializeQuickSlot`
  (`/Game/CustomContents/UI/WB_HUD.InitializeQuickSlot` (`/Game/CustomContents/Player/Blueprint/BP_PlayerController.PlayerHUD` (`self.PlayerController`)) (`self.BPC_QuickSlotSystem`)))

(event `EnhancedInput|/Game/CustomContents/Player/Inputs/IA/IA_QuickSlot3`
  (params (ActionValue :type Boolean) (ElapsedSeconds :type "Float (double-precision)") (TriggeredSeconds :type "Float (double-precision)") (InputAction :type "InputAction Object Reference" :default "/Game/CustomContents/Player/Inputs/IA/IA_QuickSlot3.IA_QuickSlot3"))
  ;[1 1 1] QuickSlotInput
  (:`Started`
    (bind _output_get (set `self.PressedQuickSlotIndex` 2))
    (`self.UseItem` _output_get)))

(event `UpdateQuickSlot`
  (`/Game/CustomContents/UI/WB_HUD.UpdateQuickSlot` (`/Game/CustomContents/Player/Blueprint/BP_PlayerController.PlayerHUD` (`self.PlayerController`)) (`self.BPC_QuickSlotSystem`)))

(event `EnhancedInput|/Game/CustomContents/Player/Inputs/IA/IA_QuickSlot4`
  (params (ActionValue :type Boolean) (ElapsedSeconds :type "Float (double-precision)") (TriggeredSeconds :type "Float (double-precision)") (InputAction :type "InputAction Object Reference" :default "/Game/CustomContents/Player/Inputs/IA/IA_QuickSlot4.IA_QuickSlot4"))
  ;[1 1 1] QuickSlotInput
  (:`Started`
    (bind _output_get (set `self.PressedQuickSlotIndex` 3))
    (`self.UseItem` _output_get)))

(event `ZoomByAiming`
  ;[1 1 1] Zoom
  (bind (_direction _springarmlength _cameraylocation) (`Timeline|Timeline` :!label _label)
    (:`Update`
      (set `SpringArmComponent.TargetArmLength` _springarmlength (`self.SpringArm`))
      (`SceneComponent.K2_SetRelativeLocation` (`self.Camera`) (`KismetMathLibrary.MakeVector` 0.0 _cameraylocation) false false))))

(event `ZoomOutByAimingEnd`
  ;[1 1 1] Zoom
  (goto _label :!via `Reverse`))

(event `EnhancedInput|/Game/CustomContents/Player/Inputs/IA/IA_QuickSlot5`
  (params (ActionValue :type Boolean) (ElapsedSeconds :type "Float (double-precision)") (TriggeredSeconds :type "Float (double-precision)") (InputAction :type "InputAction Object Reference" :default "/Game/CustomContents/Player/Inputs/IA/IA_QuickSlot5.IA_QuickSlot5"))
  ;[1 1 1] QuickSlotInput
  (:`Started`
    (bind _output_get (set `self.PressedQuickSlotIndex` 4))
    (`self.UseItem` _output_get)))

(fn `DepreciatedAddItem`
  (bind _playerhud (`/Game/CustomContents/Player/Blueprint/BP_PlayerController.PlayerHUD` (`self.PlayerController`)))
  (bind _itemimage (`/Game/CustomContents/UI/WB_HUD.ItemImage` _playerhud))
  ;[1 1 1] PickUpInput
  (bind _asbp_icon (cast `/Game/CustomContents/Items/ItemBlueprints/BP_Icon` (`|GetArrayItem` (`self.GetOverlappingActors` "/Game/CustomContents/Items/ItemBlueprints/BP_Icon.BP_Icon_C"))))
  (set `self.Icon` _asbp_icon)
  (`TextBlock.SetText` (`/Game/CustomContents/UI/WB_HUD.ItemName` _playerhud) (`KismetTextLibrary.Conv_StringToText` (`|GetEnumeratorNameAsString` (`/Game/CustomContents/Items/ItemBlueprints/BP_Icon.ItemName` (`self.Icon`)))))
  (`Image.SetBrushFromTexture` _itemimage (`/Game/CustomContents/Items/ItemBlueprints/BP_Icon.ItemImage` (`self.Icon`)) false)
  (`Image.SetColorAndOpacity` _itemimage (struct :`R` 1.0 :`G` 1.0 :`B` 1.0 :`A` 1.0))
  (`self.K2_DestroyActor` (`self.Icon`)))

(fn `GetLeftHandSocketTransform`
  (returns (LeftHandSocketTransform :type "Transform Structure"))
  (bind _weapon (`self.Weapon`)
    (:`then`
      (bind (_outposition _outrotation) (`SkinnedMeshComponent.TransformToBoneSpace` (`self.Mesh`) "hand_r" (.location (`SceneComponent.GetSocketTransform` (`/Game/CustomContents/Items/Weapons/BP_WeaponMaster.Weapon` _weapon) "LeftHandIK" "RTS_World")) (.rotation (`SceneComponent.GetSocketTransform` (`/Game/CustomContents/Items/Weapons/BP_WeaponMaster.Weapon` _weapon) "LeftHandIK" "RTS_World"))))
      (return (`KismetMathLibrary.MakeTransform` _outposition _outrotation)))
    (:`else`)))

(fn `UseConsumableItem`
  (params (StackSize :type Integer) (ItemName :type Name))
  (locals (LessAmount :type Integer) (LeastAmountItemIndex :type Integer) (SumOfItemAmount :type Integer))
  (bind (_itemname _amount) (break `/Game/CustomContents/Inventory/Blueprint/S_Slot` (`|GetArrayItem` (`/Game/CustomContents/Components/BPC_InventorySystem.Slots` (`self.BPC_InventorySystem`)) (`local.LeastAmountItemIndex`))))
  (bind _returnvalue (- _amount 1))
  (set `local.LessAmount` StackSize)
  (for (_array_element _array_index) (`/Game/CustomContents/Components/BPC_InventorySystem.Slots` (`self.BPC_InventorySystem`))
    (bind (_itemname_2 _amount_2) (break `/Game/CustomContents/Inventory/Blueprint/S_Slot` _array_element))
    (if (== (`local.ItemName`) _itemname_2)
      (if (<= _amount_2 (`local.LessAmount`))
        (set `local.LessAmount` _amount_2)
        (set `local.LeastAmountItemIndex` _array_index) ; 적다면 그 인덱스를 저장
        (else
          (set `local.LessAmount` (`local.LessAmount`))))
      (set `local.SumOfItemAmount` (+ (`local.SumOfItemAmount`) _amount_2)) ; 퀵슬롯의 아이템 전체 개수를 저장
    ))
  (if (> _returnvalue 0)
    (`KismetArrayLibrary.Array_Set` (`/Game/CustomContents/Components/BPC_InventorySystem.Slots` (`self.BPC_InventorySystem`)) (`local.LeastAmountItemIndex`) (make `/Game/CustomContents/Inventory/Blueprint/S_Slot` _itemname _returnvalue))
    (else
      (`KismetArrayLibrary.Array_Set` (`/Game/CustomContents/Components/BPC_InventorySystem.Slots` (`self.BPC_InventorySystem`)) (`local.LeastAmountItemIndex`) (make `/Game/CustomContents/Inventory/Blueprint/S_Slot` "None"))
      (if (> (- (`local.SumOfItemAmount`) 1) 0)
        (`KismetSystemLibrary.PrintString` "Keep Quick Slot")
        (else
          (for (_ _array_index_2) (`/Game/CustomContents/Components/BPC_QuickSlotSystem.QuickSlots` (`self.BPC_QuickSlotSystem`))
            (`KismetArrayLibrary.Array_Set` (`/Game/CustomContents/Components/BPC_QuickSlotSystem.QuickSlots` (`self.BPC_QuickSlotSystem`)) _array_index_2 (make `/Game/CustomContents/Inventory/Blueprint/S_Slot` "None"))))))))

(fn `UseItem`
  (params (QuickSlotIndex :type Integer))
  (bind _itemname (break `/Game/CustomContents/Inventory/Blueprint/S_Slot` (`|GetArrayItem` (`/Game/CustomContents/Components/BPC_QuickSlotSystem.QuickSlots` (`self.BPC_QuickSlotSystem`)) QuickSlotIndex)))
  (bind _returnvalue (`|GetDataTableRow` "/Game/CustomContents/Items/DT_Item.DT_Item" _itemname)
    (:`then`
      (bind ((`ItemName_6_81D54A764E1B252DC17312804880610D` _itemname_2) (`StackSize_12_4A07699846ABA4B77F2ACD8CDB8B881F` _stacksize) (`ItemType_14_F5EEFD9146030F0D2F3A7A8BDA3BBCE4` _itemtype)) (break `/Game/CustomContents/Items/ItemBlueprints/S_Item` _returnvalue))
      (set `self.Item Name` _itemname_2)
      (switch `/Game/CustomContents/Items/E_ItemType` _itemtype ; 퀵슬롯에 있는 아이템이 기본인지 소모품인지 체크
        (:`NewEnumerator4`
          (bind _returnvalue_2 (`|GetDataTableRow` "/Game/CustomContents/Items/ItemBlueprints/Consumables/DT_ConsumableItem.DT_ConsumableItem" _itemname)
            (:`then`
              (`self.UseConsumableItem` _stacksize _itemname) ; 인벤토리 슬롯과 퀵 슬롯 관리
              (`self.UpdateInventory`) ; 인벤토리 UI 업데이트
              (`self.UpdateQuickSlot`) ; 퀵슬롯 UI 업데이트
              (bind (_itemname_3 _consumableitemtype _efectpoint) (break `/Game/CustomContents/Items/ItemBlueprints/Consumables/S_ConsumableItem` _returnvalue_2))
              (switch `/Game/CustomContents/Items/ItemBlueprints/Consumables/E_ConsumableItemType` _consumableitemtype
                (:`NewEnumerator0`
                  (`/Game/CustomContents/Components/BPC_StatSystem.IncreaseHealth` (`self.BPC_StatSystem`) _efectpoint (`/Game/CustomContents/Player/Blueprint/BP_PlayerController.PlayerHUD` (`self.PlayerController`))))))))))))

(fn `UserConstructionScript`)