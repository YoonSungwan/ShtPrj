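; BP_Icon is an item actor that spins in the world and registers itself with the player while something overlaps its sphere.
; Tick plays a timeline that drives the mesh's yaw at a fixed tilt.
; Sphere overlap shows or hides the widget and sets or clears the Icon reference on the BP_Player cached at BeginPlay, without checking which actor overlapped.
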(event `self.ReceiveBeginPlay`
  (bind _asbp_player (cast `/Game/CustomContents/Player/Blueprint/BP_Player` (`GameplayStatics.GetPlayerCharacter` 0)))
  (set `self.PlayerCharacter` _asbp_player))

(event `self.ReceiveTick`
  (params (DeltaSeconds :type "Float (single-precision)"))
  (bind (_direction _angle) (`Timeline|Timeline`)
    (:`Update`
      (`SceneComponent.K2_SetRelativeRotation` (`self.Mesh`) (`KismetMathLibrary.MakeRotator` 0.0 30.0 (* _angle 180.0)) false false))))

(event `self.Sphere.OnComponentBeginOverlap`
  (params (OverlappedComponent :type "PrimitiveComponent Object Reference") (OtherActor :type "Actor Object Reference") (OtherComp :type "PrimitiveComponent Object Reference") (OtherBodyIndex :type Integer) (bFromSweep :type Boolean) (SweepResult :type "HitResult Structure (by ref)"))
  (`SceneComponent.SetVisibility` (`self.Widget`) true false)
  (set `/Game/CustomContents/Player/Blueprint/BP_Player.Icon` self (`self.PlayerCharacter`)))

(event `self.Sphere.OnComponentEndOverlap`
  (params (OverlappedComponent :type "PrimitiveComponent Object Reference") (OtherActor :type "Actor Object Reference") (OtherComp :type "PrimitiveComponent Object Reference") (OtherBodyIndex :type Integer))
  (`SceneComponent.SetVisibility` (`self.Widget`) false false)
  (set `/Game/CustomContents/Player/Blueprint/BP_Player.Icon` null (`self.PlayerCharacter`)))

(fn `UserConstructionScript`)