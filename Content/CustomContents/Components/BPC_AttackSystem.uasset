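; Player attack component that switches between an unarmed punch combo and rifle fire on the attack input.
; Montage notifies advance the four-hit combo, a timer resets it, and externally triggered, timer-driven sphere traces damage from alternating hands.
; Rifle shots trace from camera, then muzzle, applying point damage and hit reactions to BP_Enemy.
; With the rifle armed, aim input toggles zoom and crosshair.
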(event `self.ReceiveBeginPlay`
  (bind _asbp_player (cast `/Game/CustomContents/Player/Blueprint/BP_Player` (`self.GetOwner`)))
  (bind _output_get (set `self.PlayerCharacter` _asbp_player))
  (set `self.CharacterMesh` (`Character.Mesh` _output_get)))

(event `self.ReceiveTick`
  (params (DeltaSeconds :type "Float (single-precision)")))

(event `RifleFire`
  (bind _camera (`/Game/CustomContents/Player/Blueprint/BP_Player.Camera` (`self.PlayerCharacter`)))
  (bind _returnvalue (`SceneComponent.K2_GetComponentLocation` _camera))
  (bind _returnvalue_2 (`SceneComponent.GetSocketLocation` (`/Game/CustomContents/Items/Weapons/BP_WeaponMaster.Weapon` (`/Game/CustomContents/Player/Blueprint/BP_Player.Weapon` (`self.PlayerCharacter`))) "Muzzle"))
  (`self.PlayMuzzleFlash`)
  (`|PlayMontage` (`Character.Mesh` (`self.PlayerCharacter`)) "/Game/CustomContents/Animations/Montage/MM_Rifle_Fire_Montage.MM_Rifle_Fire_Montage"
    (:`then`
      (bind (_outhit _returnvalue_3) (`KismetSystemLibrary.LineTraceSingle` :`Start` _returnvalue :`End` (+ _returnvalue (* (`SceneComponent.GetForwardVector` _camera) 1000.0)) :`TraceChannel` "TraceTypeQuery1" :`DrawDebugType` "ForDuration")) ; 카메라에서 조준
      (if _returnvalue_3
        (bind (_outhit_2 _returnvalue_4) (`KismetSystemLibrary.LineTraceSingle` :`Start` _returnvalue_2 :`End` (* (`KismetMathLibrary.Normal` (- (`.ImpactPoint` (`GameplayStatics.BreakHitResult` _outhit)) _returnvalue_2)) 1000.0) :`TraceChannel` "TraceTypeQuery1" :`DrawDebugType` "ForDuration"))
        (if _returnvalue_4
          (bind (_bblockinghit _binitialoverlap _time _distance _location _impactpoint _normal _impactnormal _physmat _hitactor _hitcomponent _hitbonename) (`GameplayStatics.BreakHitResult` _outhit_2))
          (bind _asbp_enemy (cast `/Game/Blueprint/Enemy/BP_Enemy` _hitactor))
          (bind _output_get (set `/Game/Blueprint/Enemy/BP_Enemy.HitLocation` _impactpoint _asbp_enemy))
          (`GameplayStatics.ApplyPointDamage` _hitactor 10.0 _output_get _outhit_2)
          (message `/Game/Blueprint/Enemy/BPI_HitReaction.HitReaction` _hitactor _hitbonename _impactpoint))))))

(event `EnhancedInput|/Game/CustomContents/Player/Inputs/IA/IA_Attack`
  (params (ActionValue :type Boolean) (ElapsedSeconds :type "Float (double-precision)") (TriggeredSeconds :type "Float (double-precision)") (InputAction :type "InputAction Object Reference" :default "/Game/CustomContents/Player/Inputs/IA/IA_Attack.IA_Attack"))
  (bind _charactermesh (`self.CharacterMesh`))
  (:`Started`
    (if (`/Game/CustomContents/Player/Blueprint/BP_Player.IsArmedRifle` (`self.PlayerCharacter`))
      (`self.RifleFire`)
      (elif (and (not (`self.IsAttacking`)) (not (`/Game/CustomContents/Player/Blueprint/BP_Player.IsHitting` (`self.PlayerCharacter`))))
        (set `self.IsAttacking` true)
        (switch `int` (`self.ComboCounter`)
          (:`0`
            (`|PlayMontage` _charactermesh "/Game/CustomContents/Animations/Montage/Attack1_Jab_Montage.Attack1_Jab_Montage"
              (:`then`
                ;[1 1 1] 코멘트
                (`KismetSystemLibrary.K2_SetTimerDelegate` (delegate `ResetCounter`) 1.0 :!label _label))
              (:`OnInterrupted`
                (`self.ResetByHit`))
              (:`OnNotifyBegin`
                (set `self.IsAttacking` false)
                (set `self.ComboCounter` 1))))
          (:`1`
            (`|PlayMontage` _charactermesh "/Game/CustomContents/Animations/Montage/Attack2_Straight_Montage.Attack2_Straight_Montage"
              (:`then`
                (goto _label))
              (:`OnInterrupted`
                (`self.ResetByHit`))
              (:`OnNotifyBegin`
                (set `self.IsAttacking` false)
                (set `self.ComboCounter` 2))))
          (:`2`
            (`|PlayMontage` _charactermesh "/Game/CustomContents/Animations/Montage/Attack3_Hook_Montage.Attack3_Hook_Montage"
              (:`then`
                (goto _label))
              (:`OnInterrupted`
                (`self.ResetByHit`))
              (:`OnNotifyBegin`
                (set `self.IsAttacking` false)
                (set `self.ComboCounter` 3))))
          (:`3`
            (`|PlayMontage` _charactermesh "/Game/CustomContents/Animations/Montage/Attack4_Hook_Montage.Attack4_Hook_Montage"
              (:`then`
                (goto _label))
              (:`OnInterrupted`
                (`self.ResetByHit`))
              (:`OnNotifyBegin`
                (set `self.IsAttacking` false)
                (set `self.ComboCounter` 0)))))))))

(event `ResetCounter`
  ;[1 1 1] 코멘트
  (set `self.ComboCounter` 0))

(event `StopAttackTrace`
  (`KismetSystemLibrary.K2_ClearAndInvalidateTimerHandle` (`self.AttackTimerHandler`)))

(event `StartAttackTrace`
  (bind _returnvalue (`KismetSystemLibrary.K2_SetTimerDelegate` (delegate `AttackTrace`) 0.01))
  (set `self.AttackTimerHandler` _returnvalue))

(event `AttackTrace`
  (bind (_start _end) (`self.GetHandLocation` (`/Game/CustomContents/Player/Blueprint/BP_Player.LeftHand` (`self.PlayerCharacter`))))
  (bind (_start_2 _end_2) (`self.GetHandLocation` (`/Game/CustomContents/Player/Blueprint/BP_Player.RightHand` (`self.PlayerCharacter`))))
  (switch `int` (`self.ComboCounter`)
    (:`0`
      (`self.AttackSphereTrace` _start _end (`self.Base Damage`) (`self.PlayerCharacter`) :!label _label_2))
    (:`1`
      (`self.AttackSphereTrace` _start_2 _end_2 (`self.Base Damage`) (`self.PlayerCharacter`) :!label _label_3))
    (:`2`
      (goto _label_2))
    (:`3`
      (goto _label_3))))

(event `ResetByHit`
  (if (`/Game/CustomContents/Player/Blueprint/BP_Player.IsHitting` (`self.PlayerCharacter`))
    (set `self.IsAttacking` false)
    (set `self.ComboCounter` 0)))

(event `EnhancedInput|/Game/CustomContents/Player/Inputs/IA/IA_Aiming`
  (params (ActionValue :type Boolean) (ElapsedSeconds :type "Float (double-precision)") (TriggeredSeconds :type "Float (double-precision)") (InputAction :type "InputAction Object Reference" :default "/Game/CustomContents/Player/Inputs/IA/IA_Aiming.IA_Aiming"))
  ;[1 1 1] AimingInput
  (:`Triggered`
    (if (`/Game/CustomContents/Player/Blueprint/BP_Player.IsArmedRifle` (`self.PlayerCharacter`))
      (set `self.IsAiming` true)
      (set `CharacterMovementComponent.bOrientRotationToMovement` true (`Character.CharacterMovement` (`self.PlayerCharacter`)))
      (`/Game/CustomContents/Player/Blueprint/BP_Player.ZoomByAiming` (`self.PlayerCharacter`))
      (`Widget.SetVisibility` (`/Game/CustomContents/UI/WB_HUD.Crosshair` (`/Game/CustomContents/Player/Blueprint/BP_PlayerController.PlayerHUD` (`/Game/CustomContents/Player/Blueprint/BP_Player.PlayerController` (`self.PlayerCharacter`)))) "Visible")))
  (:`Canceled`
    (if (`/Game/CustomContents/Player/Blueprint/BP_Player.IsArmedRifle` (`self.PlayerCharacter`)) :!label _label_4
      (set `self.IsAiming` false)
      (set `CharacterMovementComponent.bOrientRotationToMovement` true (`Character.CharacterMovement` (`self.PlayerCharacter`)))
      (`/Game/CustomContents/Player/Blueprint/BP_Player.ZoomOutByAimingEnd` (`self.PlayerCharacter`))
      (`Widget.SetVisibility` (`/Game/CustomContents/UI/WB_HUD.Crosshair` (`/Game/CustomContents/Player/Blueprint/BP_PlayerController.PlayerHUD` (`/Game/CustomContents/Player/Blueprint/BP_Player.PlayerController` (`self.PlayerCharacter`)))) "Hidden")))
  (:`Completed`
    (goto _label_4)))

(fn `AttackSphereTrace`
  (params (Start :type "Vector Structure") (End :type "Vector Structure") (BaseDamage :type "Float (single-precision)") (DamageCauser :type "Actor Object Reference"))
  (bind (_outhit _returnvalue) (`KismetSystemLibrary.SphereTraceSingle` :`Start` Start :`End` End :`Radius` 10.0 :`TraceChannel` "TraceTypeQuery1" :`DrawDebugType` "ForDuration" :`DrawTime` 7.0))
  (if _returnvalue
    (`GameplayStatics.ApplyDamage` (`.HitActor` (`GameplayStatics.BreakHitResult` _outhit)) BaseDamage null DamageCauser)))

(fn `GetHandLocation`
  (params (self2 :type "SceneComponent Object Reference"))
  (returns (Start :type "Vector Structure") (end :type "Vector Structure"))
  (return (`SceneComponent.K2_GetComponentLocation` self2) (`KismetMathLibrary.TransformLocation` (`SceneComponent.K2_GetComponentToWorld` self2) (+ (`SceneComponent.RelativeLocation` self2) (20.0 0.0 0.0)))))

(fn `PlayMuzzleFlash`
  (bind _returnvalue (`SceneComponent.GetSocketLocation` (`/Game/CustomContents/Items/Weapons/BP_WeaponMaster.Weapon` (`/Game/CustomContents/Player/Blueprint/BP_Player.Weapon` (`self.PlayerCharacter`))) "Muzzle"))
  (`GameplayStatics.SpawnEmitterAtLocation` "/Game/MilitaryWeapDark/FX/P_AssaultRifle_MuzzleFlash.P_AssaultRifle_MuzzleFlash" _returnvalue)
  (`GameplayStatics.PlaySoundAtLocation` "/Game/MilitaryWeapDark/Sound/Rifle/RifleB_Fire_Cue.RifleB_Fire_Cue" _returnvalue (struct) 1.0 1.0 0.0 null null null null))