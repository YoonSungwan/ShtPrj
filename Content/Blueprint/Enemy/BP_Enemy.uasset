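; Zombie enemy that chases the player, attacks, and can be interrupted by hits to a weak bone.
; Detector overlap gives the player to the AI controller as target, and StartAttack sphere-traces from an arrow to damage Player-tagged actors.
; HitReaction flags an interrupt when the spine bone is hit mid-attack.
; PointDamage reduces health through the stat component, then plays death or interrupt montages and sets blackboard flags to halt the AI.
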(event `self.TempDetector.OnComponentBeginOverlap`
  (params (OverlappedComponent :type "PrimitiveComponent Object Reference") (OtherActor :type "Actor Object Reference") (OtherComp :type "PrimitiveComponent Object Reference") (OtherBodyIndex :type Integer) (bFromSweep :type Boolean) (SweepResult :type "HitResult Structure (by ref)"))
  ;[1 1 1] Chase Player in Sphere
  (bind _asbp_player (cast `/Game/CustomContents/Player/Blueprint/BP_Player` OtherActor))
  (bind _asaic_enemy (cast `/Game/Blueprint/Enemy/AIC_Enemy` (`AIBlueprintHelperLibrary.GetAIController` self)))
  (`/Game/Blueprint/Enemy/AIC_Enemy.setTarget` _asaic_enemy _asbp_player))

(event `self.ReceiveBeginPlay`
  ;[1 1 1] Set Interrupt Bone Name
  (cast `/Game/ExAsset/Zombie/ABP_Enemy` (`SkeletalMeshComponent.GetAnimInstance` (`self.Mesh`)))
  (set `self.InterruptBoneName` "Spine1")
  (`/Game/CustomContents/Components/BPC_StatSystem.Initialize Stat` (`self.BPC_StatSystem`) null))

(event `/Game/ExAsset/Pirate/Mesh_UE4/Weapon/BPI_PirateCha.HitReaction`
  (params (BoneName :type Name) (BoneLocation :type "Vector Structure"))
  ;[1 1 1] Set IsInterrupt and Hit Effect
  (`KismetSystemLibrary.PrintString` (`KismetStringLibrary.Conv_NameToString` BoneName))
  (set `self.HitLocation` BoneLocation)
  (`GameplayStatics.SpawnEmitterAtLocation` "/Game/StarterContent/Particles/P_Explosion.P_Explosion" BoneLocation)
  (set `self.IsInterrupt` (and (== BoneName (`self.InterruptBoneName`)) (`self.IsAttacking`))))

(event `self.ReceivePointDamage`
  (params (Damage :type "Float (single-precision)") (DamageType :type "DamageType Object Reference") (HitLocation :type "Vector Structure") (HitNormal :type "Vector Structure") (HitComponent :type "PrimitiveComponent Object Reference") (BoneName :type Name) (ShotFromDirection :type "Vector Structure") (InstigatedBy :type "Controller Object Reference") (DamageCauser :type "Actor Object Reference") (HitInfo :type "HitResult Structure (by ref)"))
  ;[1 1 1] Enemy Damaged and IsDead or IsInterrupt
  (set `self.Damage Causer` DamageCauser)
  (bind _isdead (`/Game/CustomContents/Components/BPC_StatSystem.DecreaseHealth` (`self.BPC_StatSystem`) Damage null))
  (if _isdead
    (`self.SetAIEnemyMoveable` (`self.IsDeadBBKey`))
    (`self.PlayAnimMontage` "/Game/ExAsset/Zombie/ZombieAnim/Montage/zombie_death_Montage.zombie_death_Montage")
    (`PrimitiveComponent.SetCollisionEnabled` (`self.CapsuleComponent`) "NoCollision")
    (`KismetSystemLibrary.Delay` 5.0)
    (`self.K2_DestroyActor`)
    (elif (`self.IsInterrupt`)
      (bind _returnvalue (`self.PlayAnimMontage` "/Game/ExAsset/Zombie/ZombieAnim/Montage/Zombie_Reaction_Hit2_Montage.Zombie_Reaction_Hit2_Montage"))
      (`self.SetAIEnemyMoveable` (`self.IsInterruptBBKey`))
      (`KismetSystemLibrary.Delay` _returnvalue)
      (set `self.IsInterrupt` false)
      (`self.SetAIEnemyMoveable` (`self.IsInterruptBBKey`) true))))

(event `StartAttack`
  (bind _hitedarrow (`self.HitedArrow`))
  ;[1 1 1] Enemy attack player
  (bind (_outhit _returnvalue) (`KismetSystemLibrary.SphereTraceSingle` :`Start` (`SceneComponent.K2_GetComponentLocation` _hitedarrow) :`End` (`KismetMathLibrary.TransformLocation` (`SceneComponent.K2_GetComponentToWorld` _hitedarrow) (+ (`SceneComponent.RelativeLocation` _hitedarrow) (10.0 0.0 0.0))) :`Radius` 10.0 :`TraceChannel` "TraceTypeQuery1" :`DrawDebugType` "ForDuration"))
  (if _returnvalue
    (bind (_bblockinghit _binitialoverlap _time _distance _location _impactpoint _normal _impactnormal _physmat _hitactor) (`GameplayStatics.BreakHitResult` _outhit))
    (if (`self.ActorHasTag` _hitactor "Player")
      (`GameplayStatics.ApplyDamage` _hitactor 10.0 null (`self.Damage Causer`)))))

(fn `SetAIEnemyMoveable`
  (params (BBKey :type Name) (Moveable :type Boolean))
  (`BlackboardComponent.SetValueAsBool` (`AIBlueprintHelperLibrary.GetBlackboard` null) BBKey (not Moveable)))

(fn `UserConstructionScript`)