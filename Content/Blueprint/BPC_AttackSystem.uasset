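; Player attack component for BP_PlayerCustom that handles melee input and weapon hit detection.
; IA_Attack plays a sword slash montage whose notify advances a timer-reset combo count, though only the first step is connected.
; StartAttackTrace sets a short non-looping timer for a debug-drawn sphere trace along the right weapon, applying damage on hit; StopAttackTrace clears it.
; The second montage and input mapping setup are disconnected.
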(event `self.ReceiveBeginPlay`
  (bind _asbp_player_custom (cast `/Game/ThirdPerson/Blueprints/BP_PlayerCustom` (`self.GetOwner`)))
  (bind _output_get (set `self.PlayerCharacter` _asbp_player_custom)))

(event `EnhancedInput|/Game/Input/IA_Attack`
  (params (ActionValue :type Boolean) (ElapsedSeconds :type "Float (double-precision)") (TriggeredSeconds :type "Float (double-precision)") (InputAction :type "InputAction Object Reference" :default "/Game/Input/IA_Attack.IA_Attack"))
  (:`Started`
    (`KismetSystemLibrary.PrintString` "Enhanced")
    (if (not (`self.Attacking`))
      (set `self.Attacking` true)
      (switch `int` (`self.ComboCount`)
        (:`0`
          (`|PlayMontage` (`self.CharacterMesh`) "/Game/ExAsset/ExAni/Sword_And_Shield_Slash_Anim_mixamo_com_Montage.Sword_And_Shield_Slash_Anim_mixamo_com_Montage"
            (:`then`
              (`KismetSystemLibrary.K2_SetTimerDelegate` (delegate `ResetCount`) 1.0))
            (:`OnNotifyBegin`
              (set `self.Attacking` false)
              (set `self.ComboCount` 1))))))))

(event `ResetCount`
  (set `self.ComboCount` 0))

(event `StartAttackTrace`
  (bind _returnvalue (`KismetSystemLibrary.K2_SetTimerDelegate` (delegate `AttackTrace`) 0.01))
  (set `self.AttackTimerHandler` _returnvalue))

(event `StopAttackTrace`
  (`KismetSystemLibrary.K2_ClearAndInvalidateTimerHandle` (`self.AttackTimerHandler`)))

(event `AttackTrace`
  (bind (_start _end) (`self.GetHandleLocation` (`/Game/ThirdPerson/Blueprints/BP_PlayerCustom.RightWeapon` (`self.PlayerCharacter`))))
  (bind (_outhit _returnvalue) (`KismetSystemLibrary.SphereTraceSingle` :`Start` _start :`End` _end :`Radius` 10.0 :`TraceChannel` "TraceTypeQuery1" :`DrawDebugType` "ForDuration" :`DrawTime` 7.0))
  (if _returnvalue
    (`GameplayStatics.ApplyDamage` (`.HitActor` (`GameplayStatics.BreakHitResult` _outhit)) 10.0 null (`self.PlayerCharacter`))))

(fn `GetHandleLocation`
  (params (Hand :type "SceneComponent Object Reference"))
  (returns (Start :type "Vector Structure") (End :type "Vector Structure"))
  (return (`SceneComponent.K2_GetComponentLocation` Hand) (`KismetMathLibrary.TransformLocation` (`SceneComponent.K2_GetComponentToWorld` Hand) (+ (`SceneComponent.RelativeLocation` Hand) (20.0 0.0 0.0)))))